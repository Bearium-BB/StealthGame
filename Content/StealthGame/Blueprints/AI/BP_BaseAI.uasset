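; BP_BaseAI is the base AI character for a stealth game, acting as the victim of takedowns.
; PlayTakedown moves it into position and plays the victim montage, whose "Ragdoll" notify stops alignment and enables mesh physics.
; UpdatePosition disables capsule collision and starts a looping timer that keeps the victim aligned to the attacker using the takedown's distance and rotation offsets.
; After a short ragdoll delay, it spawns a replacement at its starting transform and destroys itself.
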(event `self.ReceiveBeginPlay`
  (set `self.StartingPosition` (`self.GetTransform`)))

(event `/Game/StealthGame/Blueprints/BPI_TakeDownable.PlayTakedown`
  (params (Position :type "Transform Structure") (_TakedownData :type "/Game/StealthGame/ST_TakedownData Structure"))
  (bind (_takedown_data_attackermontage _takedown_data_victimmontage) (break `/Game/StealthGame/ST_TakedownData` (`self.Takedown Data`)))
  (set `self.Takedown Data` _TakedownData)
  (`self.K2_SetActorTransform` Position true true)
  (bind _notifyname (`|PlayMontage` (`self.Mesh`) _takedown_data_victimmontage)
    (:`OnNotifyBegin`
      (if (== _notifyname "Ragdoll")
        (bind _output_get (set `self.UpdatingTakedownPosition` (struct)))
        (`KismetSystemLibrary.K2_ClearAndInvalidateTimerHandle` _output_get)
        (`PrimitiveComponent.SetSimulatePhysics` (`self.Mesh`) true)
        (`KismetSystemLibrary.K2_SetTimerDelegate` (delegate `UndoTakedown`) 3.0)))))

(event `UndoTakedown`
  (`|SpawnActorFromClass` "BP_BaseAI_C" (`self.StartingPosition`) "Undefined" "MultiplyWithRoot" null null)
  (`self.K2_DestroyActor`))

(event `/Game/StealthGame/Blueprints/BPI_TakeDownable.UpdatePosition`
  (params (Actor :type "Actor Object Reference"))
  (`PrimitiveComponent.SetCollisionEnabled` (`self.CapsuleComponent`) "NoCollision")
  (set `self.TakeDownActor` Actor)
  (bind _returnvalue (`KismetSystemLibrary.K2_SetTimerDelegate` (delegate `CustomEvent`) 0.01 true true))
  (set `self.UpdatingTakedownPosition` _returnvalue))

(event `CustomEvent`
  (bind _returnvalue_location (`KismetMathLibrary.BreakTransform` (`self.GetTransform`)))
  (bind _takedown_data (`self.Takedown Data`))
  (bind (_takedown_data_attackermontage _takedown_data_victimmontage _takedown_data_alignmentdistance) (break `/Game/StealthGame/ST_TakedownData` (`self.Takedown Data`)))
  (bind _returnvalue (`self.GetTransform` (`self.TakeDownActor`)))
  (bind _returnvalue_2 (+ (* _takedown_data_alignmentdistance (`self.GetActorForwardVector` (`self.TakeDownActor`))) (`self.K2_GetActorLocation` (`self.TakeDownActor`))))
  (if (!= _returnvalue_2 _returnvalue_location)
    (`self.K2_SetActorTransform` (`KismetMathLibrary.MakeTransform` _returnvalue_2 (`KismetMathLibrary.MakeRotator` (+ (.roll (`.RotationOfVictim_14_DD2A29824312EBB2EFDB05BD7BB33C1F` (break `/Game/StealthGame/ST_TakedownData` _takedown_data))) (.roll (.rotation _returnvalue))) (+ (.pitch (`.RotationOfVictim_14_DD2A29824312EBB2EFDB05BD7BB33C1F` (break `/Game/StealthGame/ST_TakedownData` _takedown_data))) (.pitch (.rotation _returnvalue))) (+ (.yaw (`.RotationOfVictim_14_DD2A29824312EBB2EFDB05BD7BB33C1F` (break `/Game/StealthGame/ST_TakedownData` _takedown_data))) (.yaw (.rotation _returnvalue)))) (.scale _returnvalue)) true true)))

(fn `UserConstructionScript`)