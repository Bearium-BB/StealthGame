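; Grappling hook ability for the stealth game that pulls the owning character toward a surface on a rope cable created at BeginPlay.
; Releasing the input alternates through a MultiGate between tracing from the view to fire the hook and detaching it.
; A looping timer applies pull forces and updates the cable end until arrival, lost line of sight or a cutoff timer hides the cable.
; The cable-flight interpolation and slow-motion aiming are left unfinished or unwired.
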(event `self.ReceiveBeginPlay`
  (`parent.ReceiveBeginPlay`)
  (bind _returnvalue (`|AddComponentByClass` (`self.GetOwner`) "/Script/CableComponent.CableComponent" false (`KismetMathLibrary.MakeTransform` (0.0 0.0 0.0))))
  (set `self.Cable` _returnvalue)
  (`SceneComponent.SetVisibility` (`self.Cable`) false false)
  (bind _ascharacter (cast `Character` (`self.GetOwner`)))
  (set `self.Character` _ascharacter)
  (`SceneComponent.SetAbsolute` (`self.Cable`) false true false)
  (`PrimitiveComponent.SetMaterial` (`self.Cable`) 0 "/Game/StealthGame/Materials/M_Rope.M_Rope"))

(event `self.HoldInvokeAbility`
  (params (elapsedTime :type "Float (double-precision)"))
  (if (not (`self.HasBeenCanceled`))
    (`|ExecutionSequence`)))

(event `ResetMultiGate`
  (bind _charactermovement (`Character.CharacterMovement` (`self.Character`)))
  (bind (_velocity_x _velocity_y _velocity_z) (`KismetMathLibrary.BreakVector` (`MovementComponent.Velocity` _charactermovement)))
  (goto _label :!via `Reset`))

(event `self.ReleaseInvokeAbilities`
  (bind _charactermovement (`Character.CharacterMovement` (`self.Character`)))
  (bind (_velocity_x _velocity_y _velocity_z) (`KismetMathLibrary.BreakVector` (`MovementComponent.Velocity` _charactermovement)))
  (if (not (`self.HasBeenCanceled`))
    (`/Game/StealthGame/Blueprints/Abilities/BPI_BaseAbility.EndAbility`)
    (set `self.OGLocation` (`Actor.K2_GetActorLocation` (`self.Character`)))
    (`|MultiGate` false true :!label _label
      (:`Out 0`
        (bind _viewprovidertransform (message `/Game/StealthGame/Blueprints/Abilities/BPI_ViewProvider.GetViewProvider` (`self.GetOwner`)))
        (bind (_outhit _returnvalue) (`KismetSystemLibrary.LineTraceSingle` (.location _viewprovidertransform) (+ (.location _viewprovidertransform) (* 2000.0 (`KismetMathLibrary.GetForwardVector` (.rotation _viewprovidertransform)))) "TraceTypeQuery1" true (`|MakeArray` (`self.GetOwner`)) "ForDuration"))
        (if _returnvalue
          (set `self.TeleportationSpot` (`.ImpactPoint` (`GameplayStatics.BreakHitResult` _outhit)))
          (`SceneComponent.SetVisibility` (`self.Cable`) true false)
          (bind _returnvalue_2 (`KismetSystemLibrary.K2_SetTimerDelegate` :`Time` 0.01 :`bLooping` true :`bMaxOncePerFrame` true))
          (set `self.GrappleFlyingTimerHandle` _returnvalue_2)
          (`NiagaraFunctionLibrary.SpawnSystemAtLocation` "/Game/Vefects/GraplingHook/NS_GrapplingHook.NS_GrapplingHook" (`self.TeleportationSpot`))
          (`KismetSystemLibrary.K2_ClearAndInvalidateTimerHandle` (`self.GrappleFlyingTimerHandle`))
          (`KismetSystemLibrary.K2_ClearAndInvalidateTimerHandle` (`self.AddForceTimerHandle`))
          (`KismetSystemLibrary.K2_ClearAndInvalidateTimerHandle` (`self.CutOffTimerHandle`))
          (bind _returnvalue_3 (`KismetSystemLibrary.K2_SetTimerDelegate` (delegate `Add Force`) 0.01 true true))
          (`|ExecutionSequence`
            (:`then_0`
              (set `self.AddForceTimerHandle` _returnvalue_3)
              (bind _returnvalue_4 (`KismetSystemLibrary.K2_SetTimerDelegate` (delegate `CutOff`) 10.0 true true))
              (set `self.CutOffTimerHandle` _returnvalue_4)
              (`SceneComponent.SetVisibility` (`self.Cable`) true false))
            (:`then_1`
              (goto _label_3 :!via `Reset`)))
          (else
            (`self.ResetMultiGate`))))
      (:`Out 1`
        (`self.CableOff`)
        (`self.ResetMultiGate`)))))

(event `CutOff`
  (`self.CableOff`))

(event `GrappleFlying`
  (bind _cable (`self.Cable`))
  (if (< (`KismetMathLibrary.Vector_Distance` (`KismetMathLibrary.InverseTransformLocation` (`Actor.GetTransform` (`self.GetOwner`)) (`self.TeleportationSpot`)) (`KismetMathLibrary.VInterpTo` (`CableComponent.EndLocation` (`self.Cable`)) (`KismetMathLibrary.InverseTransformLocation` (`Actor.GetTransform` (`self.Character`)) (`self.TeleportationSpot`)) (`GameplayStatics.GetWorldDeltaSeconds`) 500.0)) 250.0)
    (`|ExecutionSequence`
      (:`then_0`
        (goto _label_2 :!via `Open`))
      (:`then_1`
        (`/Engine/EditorBlueprintResources/StandardMacros.Gate` true :!label _label_2
          (:`Exit`
            (`|ExecutionSequence`
              (:`then_1`
                (goto _label_2 :!via `Close`)))))))
    (else
      (set `CableComponent.EndLocation` (`KismetMathLibrary.VInterpTo` (`CableComponent.EndLocation` _cable) (`KismetMathLibrary.InverseTransformLocation` (`Actor.GetTransform` (`self.GetOwner`)) (`self.TeleportationSpot`)) (`GameplayStatics.GetWorldDeltaSeconds`) 1.0) _cable))))

(event `self.EndAbility`
  (`GameplayStatics.SetGlobalTimeDilation` 1.0))

(event `self.InvokeAbility`)

(event `self.CancelAbility`
  (set `self.HasBeenCanceled` true))

(event `Add Force`
  (bind _pullforce (`self.PullForce`))
  (bind _charactermovement (`Character.CharacterMovement` (`self.Character`)))
  (bind (_velocity_x _velocity_y _velocity_z) (`KismetMathLibrary.BreakVector` (`MovementComponent.Velocity` _charactermovement)))
  (bind (_velocity_x_2 _velocity_y_2 _velocity_z_2) (`KismetMathLibrary.BreakVector` (`MovementComponent.Velocity` (`Character.CharacterMovement` (`self.Character`)))))
  (`CharacterMovementComponent.AddImpulse` (`Character.CharacterMovement` (`self.Character`)) (0.0 0.0 2000.0) false)
  (if (`Controller.LineOfSightTo` (`GameplayStatics.GetPlayerController` 0) (`self.Character`) (`self.TeleportationSpot`) false)
    (if true
      (`|ExecutionSequence`
        (:`then_0`
          (if (< _velocity_z_2 (`self.MaxVelocityZ`))
            (`/Engine/EditorBlueprintResources/StandardMacros.DoOnce` false :!label _label_3
              (:`Completed`
                (`CharacterMovementComponent.AddImpulse` _charactermovement (`KismetMathLibrary.MakeVector` 0.0 0.0 _velocity_z) false)))))
        (:`then_1`
          (`CharacterMovementComponent.AddForce` (`Character.CharacterMovement` (`self.Character`)) (* (`KismetMathLibrary.Normal` (- (`self.TeleportationSpot`) (`Actor.K2_GetActorLocation` (`self.GetOwner`)))) (`KismetMathLibrary.MakeVector` _pullforce _pullforce 62500.0)))
          (set `CableComponent.EndLocation` (`KismetMathLibrary.InverseTransformLocation` (`Actor.GetTransform` (`self.GetOwner`)) (`self.TeleportationSpot`)) (`self.Cable`) :!label _label_4)
          (if (== (`self.TeleportationSpot`) (`Actor.K2_GetActorLocation` (`self.GetOwner`)) :`ErrorTolerance` 125.0)
            (`self.CableOff`)
            (`self.ResetMultiGate`))))
      (else
        (goto _label_4)))
    (else
      (`self.CableOff`)
      (`self.ResetMultiGate`))))

(fn `CableOff`
  (`KismetSystemLibrary.K2_ClearAndInvalidateTimerHandle` (`self.AddForceTimerHandle`))
  (`KismetSystemLibrary.K2_ClearAndInvalidateTimerHandle` (`self.CutOffTimerHandle`))
  (`SceneComponent.SetVisibility` (`self.Cable`) false false)
  (set `CharacterMovementComponent.MaxFlySpeed` 0.0 (`Character.CharacterMovement` (`self.Character`)))
  (set `CableComponent.EndLocation` (`KismetMathLibrary.MakeVector` 0.0) (`self.Cable`))
  (`NiagaraFunctionLibrary.SpawnSystemAtLocation` "/Game/Vefects/GraplingHook/NS_GrapplingHook.NS_GrapplingHook" (`self.TeleportationSpot`)))