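; BP_AbilityManager manages the owner's abilities in the stealth game and routes ability input events to the currently selected one.
; On BeginPlay it adds Grapple V2 and Blink to the owner and stores them in an array; the Bend Time setup is disconnected.
; SwitchAbillity cycles the active index, while invoke, hold, release and cancel events forward to that ability, with release also clearing its canceled flag.
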(event `SwitchAbillity`
  (`KismetSystemLibrary.PrintString` (`KismetStringLibrary.Conv_IntToString` (`self.IndexAbility`)))
  (if (> (`KismetArrayLibrary.Array_Length` (`self.Abilities`)) (+ 1 (`self.IndexAbility`)))
    (`/Engine/EditorBlueprintResources/StandardMacros.IncrementInt` (`self.IndexAbility`))
    (else
      (set `self.IndexAbility` 0))))

(event `EnhancedInput|/Game/Input/Actions/IA_CancelAbility`
  (params (ActionValue :type Boolean) (ElapsedSeconds :type "Float (double-precision)") (TriggeredSeconds :type "Float (double-precision)") (InputAction :type "InputAction Object Reference" :default "/Game/Input/Actions/IA_CancelAbility.IA_CancelAbility")))

(event `CancelAbility`
  (`/Game/StealthGame/Blueprints/Abilities/BPI_BaseAbility.CancelAbility` (`|GetArrayItem` (`self.Abilities`) (`self.IndexAbility`))))

(event `HoldInvokeAbility`
  (params (elapsedTime :type "Float (double-precision)"))
  (`/Game/StealthGame/Blueprints/Abilities/BP_BaseAbilityComponent.HoldInvokeAbility` (`|GetArrayItem` (`self.Abilities`) (`self.IndexAbility`)) elapsedTime))

(event `EnhancedInput|/Game/Input/Actions/IA_Secondary`
  (params (ActionValue :type Boolean) (ElapsedSeconds :type "Float (double-precision)") (TriggeredSeconds :type "Float (double-precision)") (InputAction :type "InputAction Object Reference" :default "/Game/Input/Actions/IA_Secondary.IA_Secondary")))

(event `InvokeAbility`
  (`/Game/StealthGame/Blueprints/Abilities/BP_BaseAbilityComponent.InvokeAbility` (`|GetArrayItem` (`self.Abilities`) (`self.IndexAbility`))))

(event `ReleaseInvokeAbilities`
  (`/Game/StealthGame/Blueprints/Abilities/BP_BaseAbilityComponent.ReleaseInvokeAbilities` (`|GetArrayItem` (`self.Abilities`) (`self.IndexAbility`)))
  (set `/Game/StealthGame/Blueprints/Abilities/BP_BaseAbilityComponent.HasBeenCanceled` false (`|GetArrayItem` (`self.Abilities`) (`self.IndexAbility`))))

(event `self.ReceiveBeginPlay`
  (bind _returnvalue (`|AddComponentByClass` (`self.GetOwner`) "/Game/StealthGame/Blueprints/Abilities/BP_GrappleV2.BP_GrappleV2_C"))
  (`KismetArrayLibrary.Array_Add` (`self.Abilities`) _returnvalue)
  (bind _returnvalue_2 (`|AddComponentByClass` (`self.GetOwner`) "/Game/StealthGame/Blueprints/Abilities/BP_Blink.BP_Blink_C"))
  (`KismetArrayLibrary.Array_Add` (`self.Abilities`) _returnvalue_2))