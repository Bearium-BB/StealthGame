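; BP_Blink is a teleport ability that moves its owner to an aimed spot in the stealth game.
; Holding traces 1000 units along the owner's view, stores the impact point offset along its normal or the trace end, and slows global time.
; Releasing restores time and teleports the owner without sweep.
; Cancelling sets a flag that blocks hold and release, without restoring time or clearing the flag here.
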(event `/Game/StealthGame/Blueprints/Abilities/BPI_BaseAbility.HoldInvokeAbility`
  (params (elapsedTime :type "Float (double-precision)"))
  (if (not (`self.HasBeenCanceled`))
    (`|ExecutionSequence`
      (:`then_0`
        (bind _viewprovidertransform (message `/Game/StealthGame/Blueprints/Abilities/BPI_ViewProvider.GetViewProvider` (`self.GetOwner`)))
        (bind (_outhit _returnvalue) (`KismetSystemLibrary.LineTraceSingle` (.location _viewprovidertransform) (+ (.location _viewprovidertransform) (* 1000.0 (`KismetMathLibrary.GetForwardVector` (.rotation _viewprovidertransform)))) "TraceTypeQuery1" false (`|MakeArray` (`self.GetOwner`)) "ForDuration"))
        (if _returnvalue
          (set `self.TeleportationSpot` (+ (`.ImpactPoint` (`GameplayStatics.BreakHitResult` _outhit)) (* (`.Normal` (`GameplayStatics.BreakHitResult` _outhit)) (`self.OppositeOfImpact`))))
          (else
            (set `self.TeleportationSpot` (`.TraceEnd` (`GameplayStatics.BreakHitResult` _outhit))))))
      (:`then_1`
        (`GameplayStatics.SetGlobalTimeDilation` 0.2)))))

(event `/Game/StealthGame/Blueprints/Abilities/BPI_BaseAbility.ReleaseInvokeAbilities`
  (if (not (`self.HasBeenCanceled`))
    (`/Game/StealthGame/Blueprints/Abilities/BPI_BaseAbility.EndAbility`)
    (`SceneComponent.K2_SetWorldLocation` (`Actor.RootComponent` (`self.GetOwner`)) (`self.TeleportationSpot`) false true)))

(event `/Game/StealthGame/Blueprints/Abilities/BPI_BaseAbility.CancelAbility`
  (set `self.HasBeenCanceled` true))

(event `/Game/StealthGame/Blueprints/Abilities/BPI_BaseAbility.EndAbility`
  (`GameplayStatics.SetGlobalTimeDilation` 1.0))

(event `/Game/StealthGame/Blueprints/Abilities/BPI_BaseAbility.InvokeAbility`)