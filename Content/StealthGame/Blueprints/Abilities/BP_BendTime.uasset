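; Bend Time ability for the stealth game that all but freezes the world while its owner keeps moving at normal speed.
; Holding the ability, unless it has been canceled, drops global time dilation to near zero and raises the owner's custom dilation to offset it.
; Cancel only sets the canceled flag; the nodes that restore normal time are unconnected, and release and end events are empty.
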(event `self.HoldInvokeAbility`
  (params (elapsedTime :type "Float (double-precision)"))
  (if (not (`self.HasBeenCanceled`))
    (`GameplayStatics.SetGlobalTimeDilation` 0.001)
    (set `Actor.CustomTimeDilation` 1000.0 (`self.GetOwner`))))

(event `self.ReleaseInvokeAbilities`)

(event `self.CancelAbility`
  (set `self.HasBeenCanceled` true))

(event `self.EndAbility`)

(event `self.InvokeAbility`)