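; Takedown manager component that triggers paired stealth takedowns between its owner and an actor found just in front of it.
; Each attempt picks from a shuffled list, requeueing the used takedown last to avoid immediate repeats.
; A sphere overlap finds the victim; both actors receive takedown data, with an alignment transform for the victim.
; A DoOnce timer enforces cooldown, cleared on a miss, and Tick feeds its progress to the HUD.
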(event `self.ReceiveBeginPlay`
  (`KismetArrayLibrary.Array_Shuffle` (`self.PossibleTakedowns`)))

(event `AttemptTakedown`
  (bind _selectedtakedown (`self.SelectedTakedown`))
  (bind (_selectedtakedown_attackermontage _selectedtakedown_victimmontage _selectedtakedown_alignmentdistance) (break `/Game/StealthGame/ST_TakedownData` (`self.SelectedTakedown`)))
  (bind _returnvalue (`Actor.GetTransform` (`self.GetOwner`)))
  (`/Engine/EditorBlueprintResources/StandardMacros.DoOnce` false :!label _label
    (:`Completed`
      (bind _returnvalue_2 (`KismetSystemLibrary.K2_SetTimerDelegate` (delegate `ResetTakedownCooldown`) (`self.TakeDownCoolDownTmer`)))
      (set `self.TimerHandlerTakedownCooldown` _returnvalue_2)
      (set `self.SelectedTakedown` (`|GetArrayItem` (`self.PossibleTakedowns`)))
      (`KismetArrayLibrary.Array_Remove` (`self.PossibleTakedowns`))
      (`KismetArrayLibrary.Array_Shuffle` (`self.PossibleTakedowns`))
      (`KismetArrayLibrary.Array_Add` (`self.PossibleTakedowns`) (`self.SelectedTakedown`))
      (bind _outactors (`KismetSystemLibrary.SphereOverlapActors` (+ (* 100.0 (`Actor.GetActorForwardVector` (`self.GetOwner`))) (`Actor.K2_GetActorLocation` (`self.GetOwner`))) 32.0 (`self.CanHit`)))
      (bind _output (`|GetArrayItem` _outactors))
      (`/Engine/EditorBlueprintResources/StandardMacros.IsValid` _output
        (:`Is Valid`
          (`KismetSystemLibrary.PrintString` (`KismetSystemLibrary.GetDisplayName` _output))
          (message `/Game/StealthGame/Blueprints/BPI_TakeDownInterfacePlayer.PlayTakedown` (`self.GetOwner`) (`self.SelectedTakedown`))
          (message `/Game/StealthGame/Blueprints/BPI_TakeDownable.PlayTakedown` _output (`KismetMathLibrary.MakeTransform` (+ (* _selectedtakedown_alignmentdistance (`Actor.GetActorForwardVector` (`self.GetOwner`))) (`Actor.K2_GetActorLocation` (`self.GetOwner`))) (`KismetMathLibrary.MakeRotator` (+ (.roll (`.RotationOfVictim_14_DD2A29824312EBB2EFDB05BD7BB33C1F` (break `/Game/StealthGame/ST_TakedownData` _selectedtakedown))) (.roll (.rotation _returnvalue))) (+ (.pitch (`.RotationOfVictim_14_DD2A29824312EBB2EFDB05BD7BB33C1F` (break `/Game/StealthGame/ST_TakedownData` _selectedtakedown))) (.pitch (.rotation _returnvalue))) (+ (.yaw (`.RotationOfVictim_14_DD2A29824312EBB2EFDB05BD7BB33C1F` (break `/Game/StealthGame/ST_TakedownData` _selectedtakedown))) (.yaw (.rotation _returnvalue)))) (.scale _returnvalue)) (`self.SelectedTakedown`))
          (message `/Game/StealthGame/Blueprints/BPI_TakeDownable.UpdatePosition` _output (`self.GetOwner`)))
        (:`Is Not Valid`
          (`KismetSystemLibrary.K2_ClearAndInvalidateTimerHandle` (`self.TimerHandlerTakedownCooldown`))
          (goto _label :!via `Reset`))))))

(event `ResetTakedownCooldown`
  (goto _label :!via `Reset`))

(event `self.ReceiveTick`
  (params (DeltaSeconds :type "Float (single-precision)"))
  (bind _asin_game_hud (cast `/Game/StealthGame/UI/Hud/InGameHUD` (`PlayerController.GetHUD` (`GameplayStatics.GetPlayerController` 0))))
  (`/Game/StealthGame/UI/Widgets/W_TakeDown.UpdateUI` (`/Game/StealthGame/UI/Hud/InGameHUD.InGameHUD` _asin_game_hud) (/ (`KismetSystemLibrary.K2_GetTimerElapsedTimeHandle` (`self.TimerHandlerTakedownCooldown`)) (`self.TakeDownCoolDownTmer`))))